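; Master Blueprint for a movable paintable object that accumulates paint splatters on its static mesh at given UV positions.
; Construction creates dynamic instances of the canvas material, applied to the mesh, and a sized splatter brush.
; BeginPlay creates and clears a single-channel R8 render target and binds it to the canvas material.
; DrawToRenderTarget sets the brush's UV location with a random blue value, then draws it into that target.
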(event Custom|DrawToRenderTarget
  (params (U :type Float%20%28single-precision%29) (V :type Float%20%28single-precision%29))
  ;[1 1 1] Draw To Render Target
  (Rendering|Material|SetVectorParameterValue (Variables|Default|GetPaintBrush) "Location" (Utilities|Struct|MakeLinearColor U V (Math|Random|RandomFloatinRange 0.0 1.0) 1.0) :!class /Script/Engine.MaterialInstanceDynamic)
  (Rendering|DrawMaterialtoRenderTarget (Variables|Default|GetRenderTarget) (Variables|Default|GetPaintBrush)))

(event EventBeginPlay
  (bind _returnvalue (Rendering|CreateRenderTarget2D (Variables|Paintable|GetRenderTargetHeight) (Variables|Paintable|GetRenderTargetWidth) "RTF_R8"))
  (bind _output_get (Variables|Default|SetRenderTarget _returnvalue))
  (Rendering|Material|SetTextureParameterValue (Variables|Default|GetPaintableMaterial) "RenderTargetTexture" _output_get)
  (Rendering|ClearRenderTarget2D (Variables|Default|GetRenderTarget)))

(fn ConstructionScript
  ;[1 1 1] Make Canvas material, Brush, and Render Target
  (bind _returnvalue (Rendering|Material|CreateDynamicMaterialInstance "/Game/Materials/MI_DefaultPaintable.MI_DefaultPaintable" :!class /Script/Engine.KismetMaterialLibrary))
  (bind _output_get (Variables|Default|SetPaintableMaterial _returnvalue))
  (Rendering|Material|SetMaterial (Variables|Default|GetStaticMesh) 0 _output_get)
  (bind _returnvalue_2 (Rendering|Material|CreateDynamicMaterialInstance "/Game/Materials/MI_SplatterBrush.MI_SplatterBrush" :!class /Script/Engine.KismetMaterialLibrary))
  (bind _output_get_2 (Variables|Default|SetPaintBrush _returnvalue_2))
  (Rendering|Material|SetScalarParameterValue _output_get_2 "BrushSize" (Variables|Paintable|GetPaintBrushSize) :!class /Script/Engine.MaterialInstanceDynamic))